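; Altar actor with a large crystal that spins every tick and seven smaller crystals that appear while something overlaps its trigger sphere.
; Sphere begin and end overlap, unfiltered by actor, toggle the small crystals through ChangeCrystalsVisibility.
; The construction script creates dynamic materials, one shared by the small crystals, and hides the sphere and its children.
; An interpolated vertical bobbing of the large crystal, using Dosmth, is present but never runs.
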(event OnComponentBeginOverlap(Sphere)
  (params (OverlappedComponent :type Primitive%20Component%20Object%20Reference) (OtherActor :type Actor%20Object%20Reference) (OtherComp :type Primitive%20Component%20Object%20Reference) (OtherBodyIndex :type Integer) (bFromSweep :type Boolean) (SweepResult :type Hit%20Result%20Structure%20%28by%20ref%29))
  (Variables|Default|SetIsPlayerInComponent true)
  (CallFunction|ChangeCrystalsVisibility true))

(event OnComponentEndOverlap(Sphere)
  (params (OverlappedComponent :type Primitive%20Component%20Object%20Reference) (OtherActor :type Actor%20Object%20Reference) (OtherComp :type Primitive%20Component%20Object%20Reference) (OtherBodyIndex :type Integer))
  (Variables|Default|SetIsPlayerInComponent false)
  (CallFunction|ChangeCrystalsVisibility false))

(event EventTick
  (params (DeltaSeconds :type Float%20%28single-precision%29))
  (Transformation|AddLocalRotation (Variables|Default|Getcrystal_Big) (Variables|Default|GetRotator) false false))

(event EventBeginPlay
  (bind _crystal_big (Variables|Default|Getcrystal_Big))
  (bind _returnvalue (Transformation|GetWorldLocation _crystal_big))
  (Variables|Default|SetMaxOffset (+ (.z _returnvalue) 5e+01))
  (Variables|Default|SetstartLocation (.z _returnvalue)))

(fn ConstructionScript
  (bind _returnvalue (Rendering|Material|CreateDynamicMaterialInstance (Variables|Default|Getcrystal_Big) 0 "/Game/lab4/materials/M_Light_2_Base_Inst1.M_Light_2_Base_Inst1" "None" :!class /Script/Engine.PrimitiveComponent))
  (bind _output_get (Variables|Default|SetCrystal_dm_big _returnvalue))
  (Rendering|Material|SetMaterial (Variables|Default|Getcrystal_Big) 0 _output_get)
  (bind _returnvalue_2 (Rendering|Material|CreateDynamicMaterialInstance (Variables|Default|Getcrystal) 0 "/Game/lab4/materials/Crystal_light.Crystal_light" "None" :!class /Script/Engine.PrimitiveComponent))
  (bind _output_get_2 (Variables|Default|SetCrystal_dm _returnvalue_2))
  (Rendering|Material|SetMaterial (Variables|Default|Getcrystal1) 0 _output_get_2)
  (Rendering|SetVisibility (Variables|Default|GetSphere) false true))

(fn ChangeCrystalsVisibility
  (params (Visible :type Boolean))
  (Rendering|SetVisibility (Variables|Default|Getcrystal1) Visible false)
  (return))

(fn Dosmth
  (bind _crystal_big (Variables|Default|Getcrystal_Big))
  (bind _startlocation (Variables|Default|GetstartLocation))
  (bind _maxoffset (Variables|Default|GetMaxOffset))
  (bind _returnvalue (Transformation|GetWorldLocation _crystal_big))
  (bind _returnvalue_2 (- _startlocation 0.0))
  (bind _returnvalue_3 (< (.z _returnvalue) _returnvalue_2))
  (if (or (> (.z _returnvalue) (- _maxoffset 1e+01)) _returnvalue_3)
    (Variables|Default|Settarget (select _returnvalue_3 _maxoffset (- _returnvalue_2 1e+01)))))