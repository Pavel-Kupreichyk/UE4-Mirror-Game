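; Actor with a pair of crystals whose glow brightens while something overlaps its Box and fades when the overlap ends.
; The construction script creates one dynamic material from Crystal_light, shares it across both crystals and starts GlowStrength at its minimum.
; Overlap events toggle a single IsActorHere flag, with no actor filtering.
; Tick steps GlowStrength toward the maximum or minimum by a fixed, frame-rate-dependent amount.
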(event OnComponentBeginOverlap(Box)
  (params (OverlappedComponent :type Primitive%20Component%20Object%20Reference) (OtherActor :type Actor%20Object%20Reference) (OtherComp :type Primitive%20Component%20Object%20Reference) (OtherBodyIndex :type Integer) (bFromSweep :type Boolean) (SweepResult :type Hit%20Result%20Structure%20%28by%20ref%29))
  (Variables|Default|SetIsActorHere true))

(event OnComponentEndOverlap(Box)
  (params (OverlappedComponent :type Primitive%20Component%20Object%20Reference) (OtherActor :type Actor%20Object%20Reference) (OtherComp :type Primitive%20Component%20Object%20Reference) (OtherBodyIndex :type Integer))
  (Variables|Default|SetIsActorHere false))

(event EventBeginPlay)

(event EventTick
  (params (DeltaSeconds :type Float%20%28single-precision%29))
  (bind _crystal_dm (Variables|Default|GetCrystal_Dm))
  (if (Variables|Default|GetIsActorHere)
    (bind _returnvalue (Rendering|Material|GetScalarParameterValue _crystal_dm "GlowStrength" :!class /Script/Engine.MaterialInstanceDynamic))
    (if (> (Variables|Default|GetGlowStrengthMax) _returnvalue)
      (Rendering|Material|SetScalarParameterValue _crystal_dm "GlowStrength" (+ _returnvalue 0.1) :!class /Script/Engine.MaterialInstanceDynamic))
    (else
      (bind _returnvalue_2 (Rendering|Material|GetScalarParameterValue _crystal_dm "GlowStrength" :!class /Script/Engine.MaterialInstanceDynamic))
      (if (> _returnvalue_2 (Variables|Default|GetGlowStrengthMin))
        (Rendering|Material|SetScalarParameterValue _crystal_dm "GlowStrength" (+ _returnvalue_2 -0.1) :!class /Script/Engine.MaterialInstanceDynamic)))))

(fn ConstructionScript
  (bind _returnvalue (Rendering|Material|CreateDynamicMaterialInstance (Variables|Default|Getcrystal) 0 "/Game/lab4/materials/Crystal_light.Crystal_light" "None" :!class /Script/Engine.PrimitiveComponent))
  (bind _output_get (Variables|Default|SetCrystal_dm _returnvalue))
  (Rendering|Material|SetMaterial (Variables|Default|Getcrystal1) 0 _output_get)
  (Rendering|Material|SetScalarParameterValue _output_get "GlowStrength" (Variables|Default|GetGlowStrengthMin) :!class /Script/Engine.MaterialInstanceDynamic))