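; Keypad actor for entering a numeric code, active only while something overlaps its trigger R.
; Digit keys append to the current input with a click sound and update a text render, while the Multiply key clears it.
; At password length, it sets IsCorrect, plays an error sound on mismatch and clears the input.
; Entering or leaving the trigger resets the display to a stored text, and leaving also clears the input.
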(event OnComponentBeginOverlap(r)
  (params (OverlappedComponent :type Primitive%20Component%20Object%20Reference) (OtherActor :type Actor%20Object%20Reference) (OtherComp :type Primitive%20Component%20Object%20Reference) (OtherBodyIndex :type Integer) (bFromSweep :type Boolean) (SweepResult :type Hit%20Result%20Structure%20%28by%20ref%29))
  (Variables|Default|SetIsInputEnabled true)
  (Rendering|Components|TextRender|SetText (Variables|Default|GetTextRender) (Variables|Default|GetNewVar_0)))

(event OnComponentEndOverlap(r)
  (params (OverlappedComponent :type Primitive%20Component%20Object%20Reference) (OtherActor :type Actor%20Object%20Reference) (OtherComp :type Primitive%20Component%20Object%20Reference) (OtherBodyIndex :type Integer))
  (Variables|Default|SetIsInputEnabled false)
  (Variables|Default|SetCurr_Input "")
  (Rendering|Components|TextRender|SetText (Variables|Default|GetTextRender) (Variables|Default|GetNewVar_0)))

(event Input|KeyboardEvents|1
  (params (Key :type Key%20Structure :default "None"))
  (:Pressed
    (if (Variables|Default|GetIsInputEnabled)
      (Variables|Default|SetCurr_Input (Utilities|String|Append (Variables|Default|GetCurr_Input) (Utilities|String|ToString(Text) (Class|KismetInputLibrary|KeyGetDisplayName Key))))
      (Audio|Components|Audio|Play (Variables|Default|GetS_Ckick) 0.0)
      (if (>= (Utilities|String|Len (Variables|Default|GetCurr_Input)) (Utilities|String|Len (Variables|Default|GetPassword)))
        (if (Utilities|Enum|Equal(Enum) (Variables|Default|GetPassword) (Variables|Default|GetCurr_Input))
          _
          (else
            (Audio|Components|Audio|Play (Variables|Default|GetS_Error) 0.0)))
        (Variables|Default|SetIsCorrect (Utilities|Enum|Equal(Enum) (Variables|Default|GetPassword) (Variables|Default|GetCurr_Input)))
        (Variables|Default|SetCurr_Input ""))
      (Rendering|Components|TextRender|SetText (Variables|Default|GetTextRender) (Utilities|Text|ToText(String) (Variables|Default|GetCurr_Input))))))

(event Input|KeyboardEvents|2
  (params (Key :type Key%20Structure :default "None"))
  (:Pressed
    (if (Variables|Default|GetIsInputEnabled)
      (Variables|Default|SetCurr_Input (Utilities|String|Append (Variables|Default|GetCurr_Input) (Utilities|String|ToString(Text) (Class|KismetInputLibrary|KeyGetDisplayName Key))))
      (Audio|Components|Audio|Play (Variables|Default|GetS_Ckick) 0.0)
      (if (>= (Utilities|String|Len (Variables|Default|GetCurr_Input)) (Utilities|String|Len (Variables|Default|GetPassword)))
        (if (Utilities|Enum|Equal(Enum) (Variables|Default|GetPassword) (Variables|Default|GetCurr_Input))
          _
          (else
            (Audio|Components|Audio|Play (Variables|Default|GetS_Error) 0.0)))
        (Variables|Default|SetIsCorrect (Utilities|Enum|Equal(Enum) (Variables|Default|GetPassword) (Variables|Default|GetCurr_Input)))
        (Variables|Default|SetCurr_Input ""))
      (Rendering|Components|TextRender|SetText (Variables|Default|GetTextRender) (Utilities|Text|ToText(String) (Variables|Default|GetCurr_Input))))))

(event Input|KeyboardEvents|Multiply
  (params (Key :type Key%20Structure :default "None"))
  (:Pressed
    (if (Variables|Default|GetIsInputEnabled)
      (Variables|Default|SetCurr_Input "")
      (Rendering|Components|TextRender|SetText (Variables|Default|GetTextRender) (Utilities|Text|ToText(String) (Variables|Default|GetCurr_Input))))))

(event Input|KeyboardEvents|0
  (params (Key :type Key%20Structure :default "None"))
  (:Pressed
    (if (Variables|Default|GetIsInputEnabled)
      (Variables|Default|SetCurr_Input (Utilities|String|Append (Variables|Default|GetCurr_Input) (Utilities|String|ToString(Text) (Class|KismetInputLibrary|KeyGetDisplayName Key))))
      (Audio|Components|Audio|Play (Variables|Default|GetS_Ckick) 0.0)
      (if (>= (Utilities|String|Len (Variables|Default|GetCurr_Input)) (Utilities|String|Len (Variables|Default|GetPassword)))
        (if (Utilities|Enum|Equal(Enum) (Variables|Default|GetPassword) (Variables|Default|GetCurr_Input))
          _
          (else
            (Audio|Components|Audio|Play (Variables|Default|GetS_Error) 0.0)))
        (Variables|Default|SetIsCorrect (Utilities|Enum|Equal(Enum) (Variables|Default|GetPassword) (Variables|Default|GetCurr_Input)))
        (Variables|Default|SetCurr_Input ""))
      (Rendering|Components|TextRender|SetText (Variables|Default|GetTextRender) (Utilities|Text|ToText(String) (Variables|Default|GetCurr_Input))))))

(event Input|KeyboardEvents|3
  (params (Key :type Key%20Structure :default "None"))
  (:Pressed
    (if (Variables|Default|GetIsInputEnabled)
      (Variables|Default|SetCurr_Input (Utilities|String|Append (Variables|Default|GetCurr_Input) (Utilities|String|ToString(Text) (Class|KismetInputLibrary|KeyGetDisplayName Key))))
      (Audio|Components|Audio|Play (Variables|Default|GetS_Ckick) 0.0)
      (if (>= (Utilities|String|Len (Variables|Default|GetCurr_Input)) (Utilities|String|Len (Variables|Default|GetPassword)))
        (if (Utilities|Enum|Equal(Enum) (Variables|Default|GetPassword) (Variables|Default|GetCurr_Input))
          _
          (else
            (Audio|Components|Audio|Play (Variables|Default|GetS_Error) 0.0)))
        (Variables|Default|SetIsCorrect (Utilities|Enum|Equal(Enum) (Variables|Default|GetPassword) (Variables|Default|GetCurr_Input)))
        (Variables|Default|SetCurr_Input ""))
      (Rendering|Components|TextRender|SetText (Variables|Default|GetTextRender) (Utilities|Text|ToText(String) (Variables|Default|GetCurr_Input))))))

(event Input|KeyboardEvents|4
  (params (Key :type Key%20Structure :default "None"))
  (:Pressed
    (if (Variables|Default|GetIsInputEnabled)
      (Variables|Default|SetCurr_Input (Utilities|String|Append (Variables|Default|GetCurr_Input) (Utilities|String|ToString(Text) (Class|KismetInputLibrary|KeyGetDisplayName Key))))
      (Audio|Components|Audio|Play (Variables|Default|GetS_Ckick) 0.0)
      (if (>= (Utilities|String|Len (Variables|Default|GetCurr_Input)) (Utilities|String|Len (Variables|Default|GetPassword)))
        (if (Utilities|Enum|Equal(Enum) (Variables|Default|GetPassword) (Variables|Default|GetCurr_Input))
          _
          (else
            (Audio|Components|Audio|Play (Variables|Default|GetS_Error) 0.0)))
        (Variables|Default|SetIsCorrect (Utilities|Enum|Equal(Enum) (Variables|Default|GetPassword) (Variables|Default|GetCurr_Input)))
        (Variables|Default|SetCurr_Input ""))
      (Rendering|Components|TextRender|SetText (Variables|Default|GetTextRender) (Utilities|Text|ToText(String) (Variables|Default|GetCurr_Input))))))

(event Input|KeyboardEvents|5
  (params (Key :type Key%20Structure :default "None"))
  (:Pressed
    (if (Variables|Default|GetIsInputEnabled)
      (Variables|Default|SetCurr_Input (Utilities|String|Append (Variables|Default|GetCurr_Input) (Utilities|String|ToString(Text) (Class|KismetInputLibrary|KeyGetDisplayName Key))))
      (Audio|Components|Audio|Play (Variables|Default|GetS_Ckick) 0.0)
      (if (>= (Utilities|String|Len (Variables|Default|GetCurr_Input)) (Utilities|String|Len (Variables|Default|GetPassword)))
        (if (Utilities|Enum|Equal(Enum) (Variables|Default|GetPassword) (Variables|Default|GetCurr_Input))
          _
          (else
            (Audio|Components|Audio|Play (Variables|Default|GetS_Error) 0.0)))
        (Variables|Default|SetIsCorrect (Utilities|Enum|Equal(Enum) (Variables|Default|GetPassword) (Variables|Default|GetCurr_Input)))
        (Variables|Default|SetCurr_Input ""))
      (Rendering|Components|TextRender|SetText (Variables|Default|GetTextRender) (Utilities|Text|ToText(String) (Variables|Default|GetCurr_Input))))))

(event Input|KeyboardEvents|6
  (params (Key :type Key%20Structure :default "None"))
  (:Pressed
    (if (Variables|Default|GetIsInputEnabled)
      (Variables|Default|SetCurr_Input (Utilities|String|Append (Variables|Default|GetCurr_Input) (Utilities|String|ToString(Text) (Class|KismetInputLibrary|KeyGetDisplayName Key))))
      (Audio|Components|Audio|Play (Variables|Default|GetS_Ckick) 0.0)
      (if (>= (Utilities|String|Len (Variables|Default|GetCurr_Input)) (Utilities|String|Len (Variables|Default|GetPassword)))
        (if (Utilities|Enum|Equal(Enum) (Variables|Default|GetPassword) (Variables|Default|GetCurr_Input))
          _
          (else
            (Audio|Components|Audio|Play (Variables|Default|GetS_Error) 0.0)))
        (Variables|Default|SetIsCorrect (Utilities|Enum|Equal(Enum) (Variables|Default|GetPassword) (Variables|Default|GetCurr_Input)))
        (Variables|Default|SetCurr_Input ""))
      (Rendering|Components|TextRender|SetText (Variables|Default|GetTextRender) (Utilities|Text|ToText(String) (Variables|Default|GetCurr_Input))))))

(event Input|KeyboardEvents|7
  (params (Key :type Key%20Structure :default "None"))
  (:Pressed
    (if (Variables|Default|GetIsInputEnabled)
      (Variables|Default|SetCurr_Input (Utilities|String|Append (Variables|Default|GetCurr_Input) (Utilities|String|ToString(Text) (Class|KismetInputLibrary|KeyGetDisplayName Key))))
      (Audio|Components|Audio|Play (Variables|Default|GetS_Ckick) 0.0)
      (if (>= (Utilities|String|Len (Variables|Default|GetCurr_Input)) (Utilities|String|Len (Variables|Default|GetPassword)))
        (if (Utilities|Enum|Equal(Enum) (Variables|Default|GetPassword) (Variables|Default|GetCurr_Input))
          _
          (else
            (Audio|Components|Audio|Play (Variables|Default|GetS_Error) 0.0)))
        (Variables|Default|SetIsCorrect (Utilities|Enum|Equal(Enum) (Variables|Default|GetPassword) (Variables|Default|GetCurr_Input)))
        (Variables|Default|SetCurr_Input ""))
      (Rendering|Components|TextRender|SetText (Variables|Default|GetTextRender) (Utilities|Text|ToText(String) (Variables|Default|GetCurr_Input))))))

(event Input|KeyboardEvents|8
  (params (Key :type Key%20Structure :default "None"))
  (:Pressed
    (if (Variables|Default|GetIsInputEnabled)
      (Variables|Default|SetCurr_Input (Utilities|String|Append (Variables|Default|GetCurr_Input) (Utilities|String|ToString(Text) (Class|KismetInputLibrary|KeyGetDisplayName Key))))
      (Audio|Components|Audio|Play (Variables|Default|GetS_Ckick) 0.0)
      (if (>= (Utilities|String|Len (Variables|Default|GetCurr_Input)) (Utilities|String|Len (Variables|Default|GetPassword)))
        (if (Utilities|Enum|Equal(Enum) (Variables|Default|GetPassword) (Variables|Default|GetCurr_Input))
          _
          (else
            (Audio|Components|Audio|Play (Variables|Default|GetS_Error) 0.0)))
        (Variables|Default|SetIsCorrect (Utilities|Enum|Equal(Enum) (Variables|Default|GetPassword) (Variables|Default|GetCurr_Input)))
        (Variables|Default|SetCurr_Input ""))
      (Rendering|Components|TextRender|SetText (Variables|Default|GetTextRender) (Utilities|Text|ToText(String) (Variables|Default|GetCurr_Input))))))

(event Input|KeyboardEvents|9
  (params (Key :type Key%20Structure :default "None"))
  (:Pressed
    (if (Variables|Default|GetIsInputEnabled)
      (Variables|Default|SetCurr_Input (Utilities|String|Append (Variables|Default|GetCurr_Input) (Utilities|String|ToString(Text) (Class|KismetInputLibrary|KeyGetDisplayName Key))))
      (Audio|Components|Audio|Play (Variables|Default|GetS_Ckick) 0.0)
      (if (>= (Utilities|String|Len (Variables|Default|GetCurr_Input)) (Utilities|String|Len (Variables|Default|GetPassword)))
        (if (Utilities|Enum|Equal(Enum) (Variables|Default|GetPassword) (Variables|Default|GetCurr_Input))
          _
          (else
            (Audio|Components|Audio|Play (Variables|Default|GetS_Error) 0.0)))
        (Variables|Default|SetIsCorrect (Utilities|Enum|Equal(Enum) (Variables|Default|GetPassword) (Variables|Default|GetCurr_Input)))
        (Variables|Default|SetCurr_Input ""))
      (Rendering|Components|TextRender|SetText (Variables|Default|GetTextRender) (Utilities|Text|ToText(String) (Variables|Default|GetCurr_Input))))))

(fn ConstructionScript)