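; Magic trap that activates when a ThirdPersonCharacter enters its capsule with a mirror state matching UseWhenInMirror.
; Activation raises four boxes from 1000 units below into place and reveals cones, particles and a spinning plane.
; With UseTime on, Tick damages the player by delta time and counts down until Deactivate lowers and hides the trap for reuse.
; Without UseTime, the trap stays active and deals no damage.
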(event OnComponentBeginOverlap(Capsule)
  (params (OverlappedComponent :type Primitive%20Component%20Object%20Reference) (OtherActor :type Actor%20Object%20Reference) (OtherComp :type Primitive%20Component%20Object%20Reference) (OtherBodyIndex :type Integer) (bFromSweep :type Boolean) (SweepResult :type Hit%20Result%20Structure%20%28by%20ref%29))
  (bind _asthird_person_character (Utilities|Casting|CastToThirdPersonCharacter OtherActor))
  (Variables|Default|Setplayer _asthird_person_character)
  (if (not (Variables|Default|GetActivated))
    (if (Math|Boolean|Equal(Boolean) (Variables|/Game/PlayerBP/Blueprints/ThirdPersonCharacter.ThirdPersonCharacter_C|GetIsinMirror _asthird_person_character) (Variables|Default|GetUseWhenInMirror?))
      (Rendering|SetVisibility (Variables|Default|GetPlane) true false)
      (Variables|Default|SetActivated true)
      (CallFunction|SetOffsetAll)
      (Rendering|SetVisibility (Variables|Default|GetNewParticleSystem) true false))))

(event EventBeginPlay
  (Variables|Default|SetLocationZ (.z (Variables|/Script/Engine.SceneComponent|GetRelativeLocation (Variables|Default|GetBox1))))
  (CallFunction|AddOffsetAll)
  (Rendering|SetVisibility (Variables|Default|GetPlane) false false)
  (Variables|Default|SetCurrTime (Variables|Default|GetTime))
  (Rendering|SetVisibility (Variables|Default|GetNewParticleSystem) false false))

(event EventTick
  (params (DeltaSeconds :type Float%20%28single-precision%29))
  (if (Variables|Default|GetActivated)
    (Transformation|AddLocalRotation (Variables|Default|GetPlane) "0,3.000000, 0" false false)
    (if (Variables|Default|GetUseTime?)
      (Default|TakeDamage (Variables|Default|Getplayer) DeltaSeconds)
      (Variables|Default|SetCurrTime (- (Variables|Default|GetCurrTime) DeltaSeconds))
      (if (<= (- (Variables|Default|GetCurrTime) DeltaSeconds) 0.0)
        (CallFunction|Deactivate)
        (Variables|Default|SetCurrTime (Variables|Default|GetTime))))))

(fn ConstructionScript)

(fn AddOffset
  (params (box :type Box%20Component%20Object%20Reference))
  (bind _relativelocation (Variables|/Script/Engine.SceneComponent|GetRelativeLocation box))
  (Transformation|SetRelativeLocation box (Math|Vector|MakeVector (.x _relativelocation) (.y _relativelocation) (- (Variables|Default|GetLocationZ) 1e+03)) false true))

(fn SetOffset
  (params (box :type Box%20Component%20Object%20Reference))
  (bind _relativelocation (Variables|/Script/Engine.SceneComponent|GetRelativeLocation box))
  (Transformation|SetRelativeLocation box (Math|Vector|MakeVector (.x _relativelocation) (.y _relativelocation) (Variables|Default|GetLocationZ)) false false))

(fn AddOffsetAll
  (CallFunction|AddOffset (Variables|Default|GetBox))
  (CallFunction|AddOffset (Variables|Default|GetBox1))
  (CallFunction|AddOffset (Variables|Default|GetBox2))
  (CallFunction|AddOffset (Variables|Default|GetBox3))
  (Rendering|SetVisibility (Variables|Default|GetCone1) false false)
  (return))

(fn SetOffsetAll
  (CallFunction|SetOffset (Variables|Default|GetBox))
  (CallFunction|SetOffset (Variables|Default|GetBox1))
  (CallFunction|SetOffset (Variables|Default|GetBox2))
  (CallFunction|SetOffset (Variables|Default|GetBox3))
  (Rendering|SetVisibility (Variables|Default|GetCone1) true false)
  (return))

(fn Deactivate
  (bind _plane (Variables|Default|GetPlane))
  (Rendering|SetVisibility _plane false false)
  (Transformation|SetRelativeRotation _plane "0, 0, 0" false false)
  (Variables|Default|SetActivated false)
  (CallFunction|AddOffsetAll)
  (Rendering|SetVisibility (Variables|Default|GetNewParticleSystem) false false))