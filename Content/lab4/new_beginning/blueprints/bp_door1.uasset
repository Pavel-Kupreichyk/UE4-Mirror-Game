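; A door actor that opens when either of its two child keypads reports a correct password, then closes itself after a countdown.
; BeginPlay casts both keypad child actors and assigns each its own password.
; Tick polls their correct flags and runs the auto-close timer.
; Open and close events play a sound and animate the door by interpolating its Z scale in short Delay loops rather than a Timeline.
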(event Custom|Open_d
  (bind _returnvalue (Utilities|Time|GetWorldDeltaSeconds))
  (bind _door_2 (Variables|Default|Getdoor_2))
  (bind _relativescale3d (Variables|/Script/Engine.SceneComponent|GetRelativeScale3D _door_2))
  (bind _returnvalue_2 (Math|Interpolation|FInterpTo (.z _relativescale3d) 0.0 _returnvalue 2.0))
  (Audio|Components|Audio|Play (Variables|Default|GetS_Open_Close) 0.0)
  (if (<= _returnvalue_2 0.1) :!label _label
    (Variables|Default|SetIsOpened true)
    (else
      (Transformation|SetRelativeScale3D _door_2 (Math|Vector|MakeVector (.x _relativescale3d) (.y _relativescale3d) _returnvalue_2))
      (Utilities|FlowControl|Delay 0.011)
      (goto _label))))

(event Custom|Close_d
  (bind _returnvalue (Utilities|Time|GetWorldDeltaSeconds))
  (bind _door_2 (Variables|Default|Getdoor_2))
  (bind _max_scale_door (Variables|Default|Getmax_scale_door))
  (bind _relativescale3d (Variables|/Script/Engine.SceneComponent|GetRelativeScale3D _door_2))
  (bind _returnvalue_2 (Math|Interpolation|FInterpTo (.z _relativescale3d) _max_scale_door _returnvalue 3.0))
  (Audio|Components|Audio|Play (Variables|Default|GetS_Open_Close) 0.0)
  (if (>= _returnvalue_2 (- _max_scale_door 0.01)) :!label _label
    (Variables|Default|SetIsOpened false)
    (Variables|Default|SetTimeToClose 1e+01)
    (else
      (Transformation|SetRelativeScale3D _door_2 (Math|Vector|MakeVector (.x _relativescale3d) (.y _relativescale3d) _returnvalue_2))
      (Utilities|FlowControl|Delay 0.01)
      (goto _label))))

(event EventBeginPlay
  (bind _asbp_keyboard (Utilities|Casting|CastTobp_keyboard (Variables|/Script/Engine.ChildActorComponent|GetChildActor (Variables|Default|Getbp_keyboard1))))
  (Variables|Default|SetKeyboard _asbp_keyboard)
  (bind _asbp_keyboard_2 (Utilities|Casting|CastTobp_keyboard (Variables|/Script/Engine.ChildActorComponent|GetChildActor (Variables|Default|Getbp_keyboard2))))
  (bind _output_get (Variables|Default|SetKeyboard2 _asbp_keyboard_2))
  (Variables|/Game/lab4/new_beginning/blueprints/bp_keyboard.bp_keyboard_C|SetPassword (Variables|Default|GetKeyboard) (Variables|Default|GetPassword1))
  (Variables|/Game/lab4/new_beginning/blueprints/bp_keyboard.bp_keyboard_C|SetPassword _output_get (Variables|Default|GetPassword2)))

(event EventTick
  (params (DeltaSeconds :type Float%20%28single-precision%29))
  (bind _keyboard (Variables|Default|GetKeyboard))
  (bind _keyboard2 (Variables|Default|GetKeyboard2))
  (Utilities|FlowControl|Sequence
    (:then_1
      (if (Variables|Default|GetIsOpened)
        (if (<= (Variables|Default|GetTimeToClose) 0.0)
          (CallFunction|CloseD)
          (else
            (Variables|Default|SetTimeToClose (- (Variables|Default|GetTimeToClose) DeltaSeconds))))
        (elif (or (Variables|/Game/lab4/new_beginning/blueprints/bp_keyboard.bp_keyboard_C|GetIsCorrect _keyboard) (Variables|/Game/lab4/new_beginning/blueprints/bp_keyboard.bp_keyboard_C|GetIsCorrect _keyboard2))
          (CallFunction|OpenD)
          (Variables|/Game/lab4/new_beginning/blueprints/bp_keyboard.bp_keyboard_C|SetIsCorrect _keyboard false)
          (Variables|/Game/lab4/new_beginning/blueprints/bp_keyboard.bp_keyboard_C|SetIsCorrect _keyboard2 false))))))

(fn ConstructionScript)