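; Healing station that spawns a Hill pickup at PlaceToSpawn and lets the player use it for healing.
; A box overlap tracks the third-person character and toggles four candle child actors' visibility.
; With no valid Hill, Tick runs the spawn timer while the player is inside, or the post-spawn cooldown regardless; leaving resets the timer.
; Pressing H inside calls HillPlayer on the spawned Hill with HillCount and plays a healing sound.
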(event OnComponentBeginOverlap(Box)
  (params (OverlappedComponent :type Primitive%20Component%20Object%20Reference) (OtherActor :type Actor%20Object%20Reference) (OtherComp :type Primitive%20Component%20Object%20Reference) (OtherBodyIndex :type Integer) (bFromSweep :type Boolean) (SweepResult :type Hit%20Result%20Structure%20%28by%20ref%29))
  (bind _asthird_person_character (Utilities|Casting|CastToThirdPersonCharacter OtherActor))
  (Variables|Default|Setplayer _asthird_person_character)
  (Variables|Default|SetActorHere? true)
  (CallFunction|SetCandleVisibility true))

(event OnComponentEndOverlap(Box)
  (params (OverlappedComponent :type Primitive%20Component%20Object%20Reference) (OtherActor :type Actor%20Object%20Reference) (OtherComp :type Primitive%20Component%20Object%20Reference) (OtherBodyIndex :type Integer))
  (Variables|Default|SetActorHere? false)
  (Variables|Default|SetCurrTime (Variables|Default|GetTimeToSpawn))
  (CallFunction|SetCandleVisibility false))

(event EventTick
  (params (DeltaSeconds :type Float%20%28single-precision%29))
  (Utilities|IsValid (Variables|Default|GetspawnedHill)
    (:Is%20Not%20Valid
      (if (Variables|Default|GetisCD?)
        (bind _output_get (Variables|Default|SetCurrTime (- (Variables|Default|GetCurrTime) DeltaSeconds)))
        (if (<= _output_get 0.0)
          (Variables|Default|SetisCD? false))
        (elif (Variables|Default|GetActorHere?)
          (bind _output_get_2 (Variables|Default|SetCurrTime (- (Variables|Default|GetCurrTime) DeltaSeconds)))
          (if (<= _output_get_2 0.0)
            (bind _returnvalue (Game|SpawnActorfromClass "/Game/lab4/new_beginning/blueprints/hill.hill_C" (Math|Conversions|ToTransform(Vector) (Transformation|GetWorldLocation (Variables|Default|GetPlaceToSpawn))) "Undefined" 0 0))
            (Variables|Default|SetspawnedHill _returnvalue)
            (Variables|Default|SetCurrTime (Variables|Default|GetTimeToSpawn))
            (Variables|Default|SetisCD? true)))))))

(event EventBeginPlay
  (Variables|Default|SetCurrTime (Variables|Default|GetTimeToSpawn))
  (CallFunction|SetCandleVisibility false))

(event Input|KeyboardEvents|H
  (params (Key :type Key%20Structure :default "None"))
  (bind _spawnedhill (Variables|Default|GetspawnedHill))
  (:Pressed
    (if (and (Variables|Default|GetActorHere?) (Utilities|IsValid _spawnedhill))
      (Default|HillPlayer _spawnedhill (Variables|Default|Getplayer) (Variables|Default|GetHillCount))
      (Audio|SpawnSoundatLocation "/Game/lab4/sounds/S_Healing.S_Healing" (Transformation|GetActorLocation) "0, 0, 0" 1.0 1.0 0.0 "/Game/lab4/new_beginning/blueprints/NewSoundAttenuation.NewSoundAttenuation" 0))))

(fn ConstructionScript)

(fn SetCandleIntensity
  (params (Intensity :type Float%20%28single-precision%29))
  (Utilities|FlowControl|Sequence
    (:then_0
      (bind _asbp_avp2_candle_tealight_naked (Utilities|Casting|CastToBP_AVP2_Candle_Tealight_Naked (Variables|/Script/Engine.ChildActorComponent|GetChildActor (Variables|Default|GetBP_AVP2_Candle_Tealight_Naked))))
      (Rendering|Components|Light|SetIntensity (Variables|/Game/ArchVisPolishPack02/Blueprints/Candles/BP_AVP2_Candle_Tealight_Naked.BP_AVP2_Candle_Tealight_Naked_C|GetPointLight _asbp_avp2_candle_tealight_naked) Intensity))
    (:then_1
      (bind _asbp_avp2_candle_tealight_naked_2 (Utilities|Casting|CastToBP_AVP2_Candle_Tealight_Naked (Variables|/Script/Engine.ChildActorComponent|GetChildActor (Variables|Default|GetBP_AVP2_Candle_Tealight_Naked1))))
      (Rendering|Components|Light|SetIntensity (Variables|/Game/ArchVisPolishPack02/Blueprints/Candles/BP_AVP2_Candle_Tealight_Naked.BP_AVP2_Candle_Tealight_Naked_C|GetPointLight _asbp_avp2_candle_tealight_naked_2) Intensity))
    (:then_2
      (bind _asbp_avp2_candle_tealight_naked_3 (Utilities|Casting|CastToBP_AVP2_Candle_Tealight_Naked (Variables|/Script/Engine.ChildActorComponent|GetChildActor (Variables|Default|GetBP_AVP2_Candle_Tealight_Naked2))))
      (Rendering|Components|Light|SetIntensity (Variables|/Game/ArchVisPolishPack02/Blueprints/Candles/BP_AVP2_Candle_Tealight_Naked.BP_AVP2_Candle_Tealight_Naked_C|GetPointLight _asbp_avp2_candle_tealight_naked_3) Intensity))
    (:then_3
      (bind _asbp_avp2_candle_tealight_naked_4 (Utilities|Casting|CastToBP_AVP2_Candle_Tealight_Naked (Variables|/Script/Engine.ChildActorComponent|GetChildActor (Variables|Default|GetBP_AVP2_Candle_Tealight_Naked3))))
      (Rendering|Components|Light|SetIntensity (Variables|/Game/ArchVisPolishPack02/Blueprints/Candles/BP_AVP2_Candle_Tealight_Naked.BP_AVP2_Candle_Tealight_Naked_C|GetPointLight _asbp_avp2_candle_tealight_naked_4) Intensity))))

(fn SetCandleVisibility
  (params (Visibility :type Boolean))
  (Rendering|SetVisibility (Variables|Default|GetBP_AVP2_Candle_Tealight_Naked) Visibility false))