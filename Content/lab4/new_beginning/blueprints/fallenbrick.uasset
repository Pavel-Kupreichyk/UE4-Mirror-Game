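; Falling brick hazard that starts dropping at BeginPlay or when a ThirdPersonCharacter overlaps its box, optionally damaging that character.
; Tick moves it down with swept SetActorLocation after an optional timeout, with optional speed increase, and destroys it below a Z limit.
; Speed is applied per frame rather than scaled by delta time.
; Non-character overlaps stop the fall, as do blocked moves against non-characters when damage is enabled.
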(event OnComponentBeginOverlap(Box1)
  (params (OverlappedComponent :type Primitive%20Component%20Object%20Reference) (OtherActor :type Actor%20Object%20Reference) (OtherComp :type Primitive%20Component%20Object%20Reference) (OtherBodyIndex :type Integer) (bFromSweep :type Boolean) (SweepResult :type Hit%20Result%20Structure%20%28by%20ref%29))
  (bind _asthird_person_character (Utilities|Casting|CastToThirdPersonCharacter OtherActor)
    (:then
      (if (Variables|Default|Getfalling?)
        (if (Variables|Default|GetaddDamage?)
          (Default|TakeDamage _asthird_person_character 3.0))
        (elif (Variables|Default|GetfallWhenOverlap?)
          (Variables|Default|Setfalling? true))))
    (:CastFailed
      (Variables|Default|Setfalling? false))))

(event EventTick
  (params (DeltaSeconds :type Float%20%28single-precision%29))
  (bind _returnvalue (Transformation|GetActorLocation))
  (if (< (.z _returnvalue) -1e+03)
    (Actor|DestroyActor)
    (elif (Variables|Default|Getfalling?)
      (if (Variables|Default|GetuseTimeOut?)
        (bind _output_get (Variables|Default|SetfallTimeOut (- (Variables|Default|GetfallTimeOut) DeltaSeconds)))
        (if (<= _output_get 0.0)
          (bind (_sweephitresult _returnvalue_2) (Transformation|SetActorLocation (Math|Vector|MakeVector (.x _returnvalue) (.y _returnvalue) (+ (.z _returnvalue) (* (Variables|Default|GetfallingSpeed) -1.0))) true false :!label _label))
          (if (Variables|Default|GetIncSpeed?)
            (Variables|Default|SetfallingSpeed (+ (Variables|Default|GetfallingSpeed) DeltaSeconds)))
          (if (not _returnvalue_2)
            (if (Variables|Default|GetaddDamage?)
              (bind _asthird_person_character (Utilities|Casting|CastToThirdPersonCharacter (.HitActor (Collision|BreakHitResult _sweephitresult)))
                (:then
                  (Default|TakeDamage _asthird_person_character (Variables|Default|Getdamage)))
                (:CastFailed
                  (Variables|Default|Setfalling? false)
                  (Variables|Default|SetfallWhenOverlap? false))))))
        (else
          (goto _label))))))

(event EventBeginPlay
  (if (Variables|Default|GetfallWhenStart?)
    (Variables|Default|Setfalling? true)))

(fn ConstructionScript)