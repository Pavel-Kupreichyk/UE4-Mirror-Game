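; Mirror-world door whose visibility and passability depend on whether the player is in the mirror or real world.
; Tick polls the ThirdPersonCharacter's IsinMirror flag and, on change, applies that world's visibility setting to SimpleDoor.
; Walkability is toggled by teleporting Box far away on local Z, or restoring its cached height to block.
; The Box overlap handler has no effect.
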(event OnComponentBeginOverlap(Box)
  (params (OverlappedComponent :type Primitive%20Component%20Object%20Reference) (OtherActor :type Actor%20Object%20Reference) (OtherComp :type Primitive%20Component%20Object%20Reference) (OtherBodyIndex :type Integer) (bFromSweep :type Boolean) (SweepResult :type Hit%20Result%20Structure%20%28by%20ref%29))
  (bind _asthird_person_character (Utilities|Casting|CastToThirdPersonCharacter OtherActor))
  (if (Variables|/Game/PlayerBP/Blueprints/ThirdPersonCharacter.ThirdPersonCharacter_C|GetIsinMirror _asthird_person_character)
    _))

(event EventBeginPlay
  (Variables|Default|SetLocationZ (.z (Variables|/Script/Engine.SceneComponent|GetRelativeLocation (Variables|Default|GetBox))))
  (bind _asthird_person_character (Utilities|Casting|CastToThirdPersonCharacter (Game|Player|GetPlayerPawn 0)))
  (Variables|Default|Setplayer _asthird_person_character)
  (Variables|Default|SetpreviosValue (not (Variables|/Game/PlayerBP/Blueprints/ThirdPersonCharacter.ThirdPersonCharacter_C|GetIsinMirror _asthird_person_character))))

(event EventTick
  (params (DeltaSeconds :type Float%20%28single-precision%29))
  (bind _player (Variables|Default|Getplayer))
  (bind _box (Variables|Default|GetBox))
  (bind _isinmirror (Variables|/Game/PlayerBP/Blueprints/ThirdPersonCharacter.ThirdPersonCharacter_C|GetIsinMirror _player))
  (bind _relativelocation (Variables|/Script/Engine.SceneComponent|GetRelativeLocation _box))
  (Utilities|IsValid _player
    (:Is%20Valid
      (if (Math|Boolean|NotEqual(Boolean) _isinmirror (Variables|Default|GetpreviosValue))
        (bind _output_get (Variables|Default|SetpreviosValue _isinmirror))
        (if _output_get
          (Rendering|SetVisibility (Variables|Default|Getsimple_door) (Variables|Default|GetVisibleWhenInMirror?) false)
          (if (Variables|Default|GetWalkableWhenInMirror?)
            (Transformation|AddLocalOffset _box (Math|Vector|MakeVector 0.0 0.0 (- (* (Variables|Default|GetLocationZ) -1e+01) 1e+03)) false true :!label _label)
            (else
              (Transformation|SetRelativeLocation _box (Math|Vector|MakeVector (.x _relativelocation) (.y _relativelocation) (Variables|Default|GetLocationZ)) false true :!label _label_2)))
          (else
            (Rendering|SetVisibility (Variables|Default|Getsimple_door) (Variables|Default|GetVisibleWhenInReal?) false)
            (if (Variables|Default|GetWalkableWhenInReal?)
              (goto _label)
              (else
                (goto _label_2)))))))))

(fn ConstructionScript)