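; Lightsaber Blueprint whose blade, MieczLight1, extends and retracts when F toggles it on and off.
; Activate and Deactivate ease the blade's uniform scale toward MaxScaleBlabe or zero with FInterpTo, re-running through short Delay loops instead of Tick or a Timeline.
; IsActivated flips only when a loop reaches its threshold.
; The construction script gives the blade a green dynamic material instance, stored in LightMaterial.
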(event Custom|Deactivate
  (bind _returnvalue (Utilities|Time|GetWorldDeltaSeconds))
  (bind _miecz_light1 (Variables|Default|Getmiecz_Light1))
  (bind _relativescale3d (Variables|/Script/Engine.SceneComponent|GetRelativeScale3D _miecz_light1))
  (bind _returnvalue_2 (Math|Interpolation|FInterpTo (.z _relativescale3d) 0.0 _returnvalue 5.0))
  (if (<= _returnvalue_2 0.01) :!label _label
    (Variables|Default|SetIsActivated false)
    (else
      (Transformation|SetRelativeScale3D _miecz_light1 (Math|Vector|MakeVector _returnvalue_2 _returnvalue_2 _returnvalue_2))
      (Utilities|FlowControl|Delay 0.01)
      (goto _label))))

(event Custom|Activate
  (bind _returnvalue (Utilities|Time|GetWorldDeltaSeconds))
  (bind _miecz_light1 (Variables|Default|Getmiecz_Light1))
  (bind _max_scale_blabe (Variables|Default|Getmax_scale_blabe))
  (bind _relativescale3d (Variables|/Script/Engine.SceneComponent|GetRelativeScale3D _miecz_light1))
  (bind _returnvalue_2 (Math|Interpolation|FInterpTo (.z _relativescale3d) _max_scale_blabe _returnvalue 5.0))
  (if (>= _returnvalue_2 (- _max_scale_blabe 0.01)) :!label _label
    (Variables|Default|SetIsActivated true)
    (else
      (Transformation|SetRelativeScale3D _miecz_light1 (Math|Vector|MakeVector _returnvalue_2 _returnvalue_2 _returnvalue_2))
      (Utilities|FlowControl|Delay 0.01)
      (goto _label))))

(event Input|KeyboardEvents|F
  (params (Key :type Key%20Structure :default "None"))
  ;[1 1 1] Move to player
  (:Pressed
    (if (Variables|Default|GetIsActivated)
      (CallFunction|Deactivate)
      (else
        (CallFunction|Activate)))))

(fn ConstructionScript
  (bind _returnvalue (Rendering|Material|CreateDynamicMaterialInstance (Variables|Default|Getmiecz_Light1) 0 "/Game/lab4/new_beginning/meshes/lightsaber/lightSaber_green.lightSaber_green" "None" :!class /Script/Engine.PrimitiveComponent))
  (Variables|Default|SetLight_material _returnvalue))