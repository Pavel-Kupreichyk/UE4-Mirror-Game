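; SpiderBP is an AI-controlled spider that reacts to the player's ThirdPersonCharacter and reports its state to its AI blackboard.
; When Pawn Sensing sees that character, it sets the player-sensed key to true.
; A capsule hit with that character marks the spider dead, in both its IsDead variable and the blackboard.
; Nothing in these graphs resets either state.
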(event OnComponentHit(CapsuleComponent)
  (params (HitComponent :type Primitive%20Component%20Object%20Reference) (OtherActor :type Actor%20Object%20Reference) (OtherComp :type Primitive%20Component%20Object%20Reference) (NormalImpulse :type Vector :default "0, 0, 0") (Hit :type Hit%20Result%20Structure%20%28by%20ref%29))
  (Utilities|Casting|CastToThirdPersonCharacter OtherActor)
  (Variables|Default|SetIsDead true)
  (AI|Components|Blackboard|SetValueasBool (AI|GetBlackboard (AI|GetAIController self)) (Variables|Default|GetIsDeadKey) true))

(event OnSeePawn(PawnSensing)
  (params (Pawn :type Pawn%20Object%20Reference))
  (Utilities|Casting|CastToThirdPersonCharacter Pawn)
  (AI|Components|Blackboard|SetValueasBool (AI|GetBlackboard (AI|GetAIController self)) (Variables|Default|GetPlayerSensedKey) true))

(fn ConstructionScript)